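; Zombie enemy character that takes damage from first-person projectiles and growls when the player comes near.
; Projectile hits reduce Health, which Tick prints on screen for debugging and polls to trigger Death below zero.
; A PlaySound overlap component plays attenuated grunts when the cached player character enters it.
; Death runs once: it plays a sound, disables collision and movement, detaches the controller, then destroys the actor after a delay.
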(event `self.ReceiveTick`
  (params (DeltaSeconds :type "Float (single-precision)"))
  ;[1 1 1] Event Tick Debug Display Health and Checks Health Condition
  (`KismetSystemLibrary.PrintString` (`KismetStringLibrary.Conv_DoubleToString` (`self.Health`)) true true (struct :`R` 0.291667 :`B` 0.00546 :`A` 1.0) DeltaSeconds)
  (if (< (`self.Health`) 0.0)
    (`self.Death`)))

(event `self.ReceiveHit`
  (params (MyComp :type "PrimitiveComponent Object Reference") (Other :type "Actor Object Reference") (OtherComp :type "PrimitiveComponent Object Reference") (bSelfMoved :type Boolean) (HitLocation :type "Vector Structure") (HitNormal :type "Vector Structure") (NormalImpulse :type "Vector Structure") (Hit :type "HitResult Structure (by ref)"))
  ;[1 1 1] When Projectile Hits; -10 Health
  (if (`.bSuccess` (castclass `/Game/FirstPersonBP/Blueprints/FirstPersonProjectile` (`GameplayStatics.GetObjectClass` Other) :!pure true))
    (set `self.Health` (- (`self.Health`) 13.0))))

(event `self.ReceiveBeginPlay`
  ;[1 1 1] On Begin Play; Set Health and Fisrt Person Character Reference
  (set `self.Health` 100.0)
  (bind _asfirst_person_character (cast `/Game/FirstPersonBP/Blueprints/FirstPersonCharacter` (`GameplayStatics.GetPlayerPawn` 0)))
  (set `self.First Person Character Reference` _asfirst_person_character))

(event `self.PlaySound.OnComponentBeginOverlap`
  (params (OverlappedComponent :type "PrimitiveComponent Object Reference") (OtherActor :type "Actor Object Reference") (OtherComp :type "PrimitiveComponent Object Reference") (OtherBodyIndex :type Integer) (bFromSweep :type Boolean) (SweepResult :type "HitResult Structure (by ref)"))
  ;[1 1 1] Play Grunt/Chase Sound when near player
  (if (== OtherActor (`self.First Person Character Reference`))
    (`GameplayStatics.PlaySoundAtLocation` "/Game/DV-Zombie/DV-Zombie_Sounds/Grunts_Cue.Grunts_Cue" (`SceneComponent.K2_GetComponentLocation` (`self.CapsuleComponent`)) (struct) 1.0 1.0 0.0 "/Game/DV-Zombie/DV-Zombie_Sounds/Zombie_Death_Sound_Attenuation.Zombie_Death_Sound_Attenuation" null null)))

(event `Death`
  ;[1 1 1] Death Event
  (`/Engine/EditorBlueprintResources/StandardMacros.DoOnce` false
    (:`Completed`
      (`GameplayStatics.PlaySoundAtLocation` "/Game/DV-Zombie/DV-Zombie_Sounds/MonsterDeathFinal_Cue.MonsterDeathFinal_Cue" (`SceneComponent.K2_GetComponentLocation` (`self.CapsuleComponent`)) (struct) 1.0 1.0 0.0 "/Game/DV-Zombie/DV-Zombie_Sounds/Zombie_Death_Sound_Attenuation.Zombie_Death_Sound_Attenuation" null null)
      (`PrimitiveComponent.SetCollisionEnabled` (`self.CapsuleComponent`) "NoCollision")
      (`CharacterMovementComponent.DisableMovement` (`self.CharacterMovement`))
      (`self.DetachFromControllerPendingDestroy`)
      (`KismetSystemLibrary.Delay` 5.0)
      (`self.K2_DestroyActor`))))

(fn `UserConstructionScript`)